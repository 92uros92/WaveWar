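; BP_ShadowPlayerController is the player controller that opens the in-game menu when Tab is pressed.
; Tab creates a game menu layout widget, adds it to the viewport, and registers it as the MainMenuSubsystem's primary layout.
; It then pushes the game menu screen, looked up by gameplay tag, onto the GameMenu stack as a soft widget class.
; After the push, it switches to UI-only input, shows the cursor and pauses the game.
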(event EventBeginPlay)

(event EventTick
  (params (DeltaSeconds :type Float%20%28single-precision%29)))

(event Input|KeyboardEvents|Tab
  (params (Key :type Key%20Structure :default "None"))
  (:Pressed
    (bind _returnvalue (UserInterface|CreateWidget "/Game/Blueprints/UI/MainMenu/GameMenu/WBP_GameMenuLayout.WBP_GameMenuLayout_C" self))
    (UserInterface|Viewport|AddtoViewport _returnvalue 0)
    (Class|MainMenuSubsystem|InitializePrimaryLayoutWidget (Subsystems|GetMainMenuSubsystem) _returnvalue)
    (|PushSoftWidget self (Class|WWBlueprintFunctionLibrary|GetMainMenuClassbyTag "(TagName=\"Menu.Widget.GameMenuScreen\")") "(TagName=\"GameMenu.Stack.GameMenu\")" true
      (:then
        (Input|SetInputModeUIOnly self 0 "DoNotLock" false)
        (Variables|Default|SetbShowMouseCursor true)
        (Game|SetGamePaused true)))))

(fn ConstructionScript)