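; Base enemy Blueprint that handles turn-to-target motion warping and loot spawning.
; UpdateTurntoTarget feeds the given location into Motion Warping as the TurnToTarget warp target.
; SpawnLoot stores the list returned by GetLootItem, then spawns only its first entry's class at the enemy's transform, and only for the Fighter character class.
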(event EventBeginPlay)

(event Collision|EventActorBeginOverlap
  (params (OtherActor :type Actor%20Object%20Reference)))

(event EventTick
  (params (DeltaSeconds :type Float%20%28single-precision%29)))

(event EventSpawnLoot
  (bind _returnvalue (Class|WWBlueprintFunctionLibrary|GetLootItem))
  (Utilities|IsValid _returnvalue
    (:Is%20Valid
      (bind _returnvalue_2 (Class|LootData|GetLootItem _returnvalue))
      (bind _output_get (Variables|Default|SetLootItems _returnvalue_2))
      (if (Utilities|Array|IsValidIndex _output_get)
        (if (Utilities|Enum|Equal(Enum) (Variables|Default|GetCharacterClass) "Fighter")
          (Game|SpawnActorfromClass (.LootClass (Utilities|Struct|BreakLootItem (Utilities|Array|Get(acopy) _output_get))) (Transformation|GetActorTransform) "AlwaysSpawn" "MultiplyWithRoot" 0 0))))))

(event EventUpdateTurntoTarget
  (params (Target :type Vector%20%28by%20ref%29 :default "0, 0, 0"))
  (Class|MotionWarpingComponent|AddorUpdateWarpTargetfromLocation (Variables|Default|GetMotionWarping) "TurnToTarget" Target))

(fn ConstructionScript)