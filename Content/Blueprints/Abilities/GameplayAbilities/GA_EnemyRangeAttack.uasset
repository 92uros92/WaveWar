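; Enemy ranged attack gameplay ability, currently without any damage or projectile logic.
; On activation it plays a random montage from the avatar's CombatInterface and waits for that montage's gameplay event tag.
; The event triggers a small sphere query at the tag's socket for live players and checks their team, but takes no action on hits.
; The ability ends after that query, when the montage finishes or is interrupted, or if no montages exist.
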(event Ability|EventActivateAbility
  (bind _returnvalue (Ability|GetAvatarActorfromActorInfo))
  (bind _returnvalue_2 (Ability|GetAvatarActorfromActorInfo))
  (Utilities|Casting|CastToCombatInterface _returnvalue)
  (bind _returnvalue_3 (Class|CombatInterface|GetAttackMontages(Message) _returnvalue))
  (bind _output_get (Variables|Default|SetTaggedMontage (Utilities|Array|Get(acopy) _returnvalue_3 (Math|Random|RandomIntegerinRange 0 (- (Utilities|Array|Length _returnvalue_3) 1)))))
  (if (> (Utilities|Array|Length _returnvalue_3) 0)
    (|PlayMontageandWaitProxy "None" (.Montage (Utilities|Struct|BreakMontageForAttack _output_get)) 1.0 "None" false 1.0 0.0 false
      (:then
        (Ability|Tasks|WaitGameplayEvent (.MontageTag (Utilities|Struct|BreakMontageForAttack _output_get)) 0
          (:EventReceived
            (bind _returnvalue_4 (Class|CombatInterface|GetSocketLocation(Message) _returnvalue_2 (.MontageTag (Utilities|Struct|BreakMontageForAttack _output_get))))
            (bind _outoverlappingactors (Class|ShadowGameMode|GetLivePlayersinRadius _returnvalue_2 (Utilities|Array|MakeArray _returnvalue_2) 45.0 _returnvalue_4))
            (for _array_element _outoverlappingactors
              (if (Class|WWBlueprintFunctionLibrary|IsNotSameTeam (Ability|GetAvatarActorfromActorInfo) _array_element)
                _))
            (Ability|EndAbility))))
      (:OnCompleted
        (Ability|EndAbility :!label _label))
      (:OnInterrupted
        (goto _label))
      (:OnCancelled
        (goto _label)))
    (else
      (goto _label))))

(event Ability|EventOnEndAbility
  (params (bWasCancelled :type Boolean)))